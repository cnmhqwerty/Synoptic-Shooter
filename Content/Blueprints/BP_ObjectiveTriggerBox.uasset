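; BP_ObjectiveTriggerBox is a capture-point volume that builds up the player's capture progress while they stand inside it.
; Begin and end overlap toggle HoldingPoint on any overlapping BP_FirstPersonCharacter.
; Tick adds a fixed step to CapAmount, clamped to MaxCap, but only for player 0's character cached at BeginPlay.
; The increment ignores delta time, so capture speed depends on frame rate, and progress never decays here.
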(event EventBeginPlay
  (bind _asbp_first_person_character (Utilities|Casting|CastToBP_FirstPersonCharacter (Game|GetPlayerCharacter 0)))
  (Variables|Default|SetAs%20BP%20First%20Person%20Character _asbp_first_person_character))

(event EventTick
  (params (DeltaSeconds :type Float%20%28single-precision%29))
  (bind _as_bp_first_person_character (Variables|Default|GetAs%20BP%20First%20Person%20Character))
  (if (Variables|/Game/FirstPerson/Blueprints/BP_FirstPersonCharacter.BP_FirstPersonCharacter_C|GetHoldingPoint (Variables|Default|GetAs%20BP%20First%20Person%20Character))
    (Variables|/Game/FirstPerson/Blueprints/BP_FirstPersonCharacter.BP_FirstPersonCharacter_C|SetCapAmount _as_bp_first_person_character (Math|Float|Clamp(Float) (+ (Variables|/Game/FirstPerson/Blueprints/BP_FirstPersonCharacter.BP_FirstPersonCharacter_C|GetCapAmount _as_bp_first_person_character) 0.1) 0.0 (Variables|/Game/FirstPerson/Blueprints/BP_FirstPersonCharacter.BP_FirstPersonCharacter_C|GetMaxCap _as_bp_first_person_character)))))

(event Collision|EventActorBeginOverlap
  (params (OtherActor :type Actor%20Object%20Reference))
  (bind _asbp_first_person_character (Utilities|Casting|CastToBP_FirstPersonCharacter OtherActor))
  (Variables|/Game/FirstPerson/Blueprints/BP_FirstPersonCharacter.BP_FirstPersonCharacter_C|SetHoldingPoint _asbp_first_person_character true))

(event Collision|EventActorEndOverlap
  (params (OtherActor :type Actor%20Object%20Reference))
  (bind _asbp_first_person_character (Utilities|Casting|CastToBP_FirstPersonCharacter OtherActor))
  (Variables|/Game/FirstPerson/Blueprints/BP_FirstPersonCharacter.BP_FirstPersonCharacter_C|SetHoldingPoint _asbp_first_person_character false))

(fn ConstructionScript)