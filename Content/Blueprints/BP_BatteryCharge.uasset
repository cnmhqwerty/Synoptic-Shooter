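; BP_BatteryCharge is a battery charge indicator whose mesh grows vertically while the first-person character's HoldingPoint flag is set.
; Each Tick casts player 0 to BP_FirstPersonCharacter and adds its CapAmount/MaxCap ratio, divided by twice MaxHeight, to the mesh's world Z scale.
; Z scale is clamped between zero and MaxHeight, and the increment accumulates per frame without delta-time scaling.
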(event EventBeginPlay)

(event Collision|EventActorBeginOverlap
  (params (OtherActor :type Actor%20Object%20Reference)))

(event EventTick
  (params (DeltaSeconds :type Float%20%28single-precision%29))
  (bind _self self)
  (bind _maxheight (Variables|Default|GetMaxHeight))
  (bind _staticmeshcomponent (Variables|Debug|GetStaticMeshComponent _self))
  (bind _asbp_first_person_character (Utilities|Casting|CastToBP_FirstPersonCharacter (Game|GetPlayerCharacter 0)))
  (if (Variables|/Game/FirstPerson/Blueprints/BP_FirstPersonCharacter.BP_FirstPersonCharacter_C|GetHoldingPoint _asbp_first_person_character)
    (Transformation|SetWorldScale3D _staticmeshcomponent (Math|Vector|MakeVector (.x (+ (Transformation|GetWorldScale _staticmeshcomponent) (Math|Vector|MakeVector 0.0 0.0 (/ (/ (Variables|/Game/FirstPerson/Blueprints/BP_FirstPersonCharacter.BP_FirstPersonCharacter_C|GetCapAmount _asbp_first_person_character) (Variables|/Game/FirstPerson/Blueprints/BP_FirstPersonCharacter.BP_FirstPersonCharacter_C|GetMaxCap _asbp_first_person_character)) (* _maxheight 2.0))))) (.y (+ (Transformation|GetWorldScale _staticmeshcomponent) (Math|Vector|MakeVector 0.0 0.0 (/ (/ (Variables|/Game/FirstPerson/Blueprints/BP_FirstPersonCharacter.BP_FirstPersonCharacter_C|GetCapAmount _asbp_first_person_character) (Variables|/Game/FirstPerson/Blueprints/BP_FirstPersonCharacter.BP_FirstPersonCharacter_C|GetMaxCap _asbp_first_person_character)) (* _maxheight 2.0))))) (Math|Float|Clamp(Float) (.z (+ (Transformation|GetWorldScale _staticmeshcomponent) (Math|Vector|MakeVector 0.0 0.0 (/ (/ (Variables|/Game/FirstPerson/Blueprints/BP_FirstPersonCharacter.BP_FirstPersonCharacter_C|GetCapAmount _asbp_first_person_character) (Variables|/Game/FirstPerson/Blueprints/BP_FirstPersonCharacter.BP_FirstPersonCharacter_C|GetMaxCap _asbp_first_person_character)) (* _maxheight 2.0))))) 0.0 _maxheight)))))

(fn ConstructionScript)