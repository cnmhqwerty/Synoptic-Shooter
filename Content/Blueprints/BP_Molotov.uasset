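; BP_Molotov is a fire damage area that repeatedly hurts enemies standing inside it.
; Begin and end overlap events add and remove BP_Enemy_Base actors in the InFire array, ignoring all other actors.
; Tick applies MolotovDamage to every actor in that array, throttled to roughly ten hits per second by a DoOnce that resets after a short Delay.
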(event Collision|EventActorBeginOverlap
  (params (OtherActor :type Actor%20Object%20Reference))
  (bind _asbp_enemy_base (Utilities|Casting|CastToBP_Enemy_Base OtherActor))
  (Utilities|Array|Add (Variables|Default|GetInFire) _asbp_enemy_base))

(event EventTick
  (params (DeltaSeconds :type Float%20%28single-precision%29))
  (Utilities|FlowControl|DoOnce false :!label _label
    (:Completed
      (for _array_element (Variables|Default|GetInFire)
        (Game|Damage|ApplyDamage _array_element (Variables|Default|GetMolotovDamage) 0 0))
      (Utilities|FlowControl|Delay 0.1)
      (goto _label Reset))))

(event Collision|EventActorEndOverlap
  (params (OtherActor :type Actor%20Object%20Reference))
  (bind _asbp_enemy_base (Utilities|Casting|CastToBP_Enemy_Base OtherActor))
  (Utilities|Array|RemoveItem (Variables|Default|GetInFire) _asbp_enemy_base))

(fn ConstructionScript)