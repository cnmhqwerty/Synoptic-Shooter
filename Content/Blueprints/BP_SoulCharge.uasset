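; Soul charge Blueprint that visualizes the player's CapAmount as a static mesh that grows vertically on pickup.
; On BeginPlay it caches the player and starts an endless one-second delay loop that drains CapAmount, clamped between zero and one.
; OnPickup prints a debug message and adds CapAmount divided by MaxHeight to the mesh's world Z scale, capped at MaxHeight.
; The drain loop never shrinks the mesh.
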(event Custom|OnPickup
  (bind _self self)
  (bind _maxheight (Variables|Default|GetMaxHeight))
  (bind _staticmeshcomponent (Variables|Debug|GetStaticMeshComponent _self))
  (Development|PrintString "Increase")
  (Transformation|SetWorldScale3D _staticmeshcomponent (Math|Vector|MakeVector (.x (+ (Transformation|GetWorldScale _staticmeshcomponent) (Math|Vector|MakeVector 0.0 0.0 (/ (Variables|/Game/Player/BP_FirstPersonCharacter.BP_FirstPersonCharacter_C|GetCapAmount (stale EventBeginPlay _asbp_first_person_character)) _maxheight)))) (.y (+ (Transformation|GetWorldScale _staticmeshcomponent) (Math|Vector|MakeVector 0.0 0.0 (/ (Variables|/Game/Player/BP_FirstPersonCharacter.BP_FirstPersonCharacter_C|GetCapAmount (stale EventBeginPlay _asbp_first_person_character)) _maxheight)))) (Math|Float|Clamp(Float) (.z (+ (Transformation|GetWorldScale _staticmeshcomponent) (Math|Vector|MakeVector 0.0 0.0 (/ (Variables|/Game/Player/BP_FirstPersonCharacter.BP_FirstPersonCharacter_C|GetCapAmount (stale EventBeginPlay _asbp_first_person_character)) _maxheight)))) 0.0 _maxheight))))

(event EventBeginPlay
  (bind _asbp_first_person_character (Utilities|GetPlayer))
  (Utilities|FlowControl|Delay 1.0 :!label _label)
  (Variables|/Game/Player/BP_FirstPersonCharacter.BP_FirstPersonCharacter_C|SetCapAmount _asbp_first_person_character (Math|Float|Clamp(Float) (- (Variables|/Game/Player/BP_FirstPersonCharacter.BP_FirstPersonCharacter_C|GetCapAmount _asbp_first_person_character) 0.5)))
  (goto _label))

(fn ConstructionScript)