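; BP_Enemy_Base is a base enemy that takes damage from the player and drops an objective pickup on death.
; One tick after BeginPlay it caches the player and binds to OnTakeAnyDamage.
; Only damage instigated by the player reduces Health.
; At zero or below, it spawns BP_Objective_Pickup at the mesh's world transform and destroys itself.
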(event Custom|OnDeath
  (Game|SpawnActorfromClass "/Game/Blueprints/BP_Objective_Pickup.BP_Objective_Pickup_C" (Transformation|GetWorldTransform (Variables|Character|GetMesh)) "AdjustIfPossibleButAlwaysSpawn" "MultiplyWithRoot" 0 0)
  (Actor|DestroyActor))

(event Custom|HitByPlayer
  (params (DamagedActor :type Actor%20Object%20Reference) (Damage :type Float%20%28single-precision%29) (DamageType :type Damage%20Type%20Object%20Reference) (InstigatedBy :type Controller%20Object%20Reference) (DamageCauser :type Actor%20Object%20Reference))
  (if (== InstigatedBy (Variables|Default|GetPlayer))
    (bind _output_get (Variables|Default|SetHealth (- (Variables|Default|GetHealth) Damage)))
    (if (<= _output_get 0.0)
      (CallFunction|OnDeath))))

(event EventBeginPlay
  (Utilities|FlowControl|DelayUntilNextTick)
  (bind _asbp_first_person_character (Utilities|GetPlayer))
  (Variables|Default|SetPlayer _asbp_first_person_character)
  (EventDispatchers|BindEventtoOnTakeAnyDamage (delegate Custom|HitByPlayer)))

(fn ConstructionScript)