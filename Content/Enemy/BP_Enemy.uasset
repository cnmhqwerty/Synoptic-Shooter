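; Enemy Blueprint that performs a punch attack against the player.
; BeginPlay waits one tick, then caches the player reference.
; Attack plays the punch montage on the mesh and, whether it completes or is interrupted, applies damage to the cached player and calls the attack-end notification.
; Damage lands when the montage ends, with no range or hit check in this graph.
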(event Custom|Attack
  (Animation|Montage|PlayMontage (Variables|Character|GetMesh) "/Game/Enemy/Animations/AM_EnemyPunch.AM_EnemyPunch"
    (:OnCompleted
      _)
    (:OnInterrupted
      _))
  (Game|Damage|ApplyDamage (Variables|Default|GetPlayer) (Variables|Default|GetDamageDealt) 0 self "/Script/Engine.DamageType")
  (Default|CallOnAttackEnd))

(event EventBeginPlay
  (Utilities|FlowControl|DelayUntilNextTick)
  (bind _asbp_first_person_character (Utilities|GetPlayer))
  (Variables|Default|SetPlayer _asbp_first_person_character))

(event Collision|EventActorBeginOverlap
  (params (OtherActor :type Actor%20Object%20Reference)))

(fn ConstructionScript)