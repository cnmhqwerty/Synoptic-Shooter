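; Melee enemy that extends a parent enemy Blueprint with a punch attack against the player.
; The Attack event plays the punch montage, then applies damage if the player is within a fixed distance when the montage completes or is interrupted.
; Both outcomes then fire the OnAttackEnd dispatcher, whether or not damage landed.
; The hit is a plain distance check, with no trace or collision test.
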(event Custom|Attack
  (bind _self self)
  (bind _player (Variables|Default|GetPlayer))
  (Animation|Montage|PlayMontage (Variables|Character|GetMesh) "/Game/Enemy/Animations/AM_EnemyPunch.AM_EnemyPunch"
    (:OnCompleted
      _)
    (:OnInterrupted
      _))
  (if (< (Transformation|GetDistanceTo _player _self) 3e+02)
    (Game|Damage|ApplyDamage _player (Variables|Default|GetDamageDealt) 0 _self "/Script/Engine.DamageType"))
  (Default|CallOnAttackEnd))

(event EventBeginPlay
  (|CallParentFunction))

(event Collision|EventActorBeginOverlap
  (params (OtherActor :type Actor%20Object%20Reference))
  (|CallParentFunction OtherActor) ; This node is disabled and will not be called.\nDrag off pins to build functionality.
)

(event EventTick
  (params (DeltaSeconds :type Float%20%28single-precision%29)))

(fn ConstructionScript
  (|CallParentFunction))