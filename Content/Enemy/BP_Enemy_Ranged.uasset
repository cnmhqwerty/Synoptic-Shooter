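; BP_Enemy_Ranged is an enemy that attacks the player by shooting projectiles.
; On BeginPlay it adds a projectile weapon component at runtime and keeps a reference to it.
; Each Attack aims from the capsule toward the player's root location with a look-at rotation, fires the weapon, then immediately signals the attack end.
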(event Custom|Attack
  (bind _asbp_first_person_character (Utilities|GetPlayer))
  (Default|Shoot (stale EventBeginPlay _returnvalue) (Math|Rotator|FindLookatRotation (Transformation|GetWorldLocation (Variables|Default|GetCapsuleComponent)) (Transformation|GetWorldLocation (Variables|/Script/Engine.Actor|GetRootComponent _asbp_first_person_character))))
  (Default|CallOnAttackEnd))

(event EventBeginPlay
  (|CallParentFunction)
  (bind _returnvalue (AddComponent|AddBPEnemyProjectileWeaponComponent false)))

(event Collision|EventActorBeginOverlap
  (params (OtherActor :type Actor%20Object%20Reference))
  (|CallParentFunction OtherActor) ; This node is disabled and will not be called.\nDrag off pins to build functionality.
)

(fn ConstructionScript
  (|CallParentFunction))